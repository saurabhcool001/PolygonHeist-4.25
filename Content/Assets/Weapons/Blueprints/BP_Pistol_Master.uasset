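; Master pistol weapon Blueprint that handles the cosmetic side of firing and reloading, with no trace, damage or ammo logic.
; FirePistol plays a sound cue and muzzle-flash emitter at the Muzzle socket, ejects an empty case actor from EjectionPort and plays the fire animation on the skeletal mesh.
; ReloadMagazine only spawns a dropped-magazine actor at the Magazine socket.
; The fire sound references a flesh-impact cue rather than a gunshot.
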(event `Fire Pistol`
  (bind _skeletalmesh (`self.SkeletalMesh`))
  (bind _returnvalue (`SceneComponent.GetSocketLocation` _skeletalmesh (`self.Muzzle`)))
  (`GameplayStatics.PlaySoundAtLocation` "/Game/Assets/Audio/Effects/bullet_impact_body_flesh_01_Cue.bullet_impact_body_flesh_01_Cue" _returnvalue (struct) 1.0 1.0 0.0 null null null)
  (`GameplayStatics.SpawnEmitterAtLocation` "/Game/PolygonHeist/ParticleFX/FX_Gunshot.FX_Gunshot" _returnvalue (`SceneComponent.GetSocketRotation` _skeletalmesh (`self.Muzzle`)))
  (`|SpawnActorFromClass` "/Game/Assets/Weapons/Pickups/BP_Pistol_Empty_Case.Bp_Pistol_Empty_Case_C" (`SceneComponent.GetSocketTransform` _skeletalmesh (`self.Ejection Port`) "RTS_World") "Undefined" "OverrideRootScale" null null)
  (`SkeletalMeshComponent.PlayAnimation` (`self.SkeletalMesh`) "/Game/Assets/Weapons/Blueprints/SWAT_P_Fire.SWAT_P_Fire" false))

(event `Reload Magazine`
  (`|SpawnActorFromClass` "/Game/Assets/Weapons/Pickups/BP_Pistol_Mag_Drop.BP_Pistol_Mag_Drop_C" (`SceneComponent.GetSocketTransform` (`self.SkeletalMesh`) (`self.Magazine`) "RTS_World") "Undefined" "OverrideRootScale" null null))

(fn `UserConstructionScript`)