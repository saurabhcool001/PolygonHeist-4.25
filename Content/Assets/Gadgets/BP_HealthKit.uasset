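; BP_HealthKit is a health pickup that heals a BP_Player_Base overlapping its pickup area, unless Health is exactly 100.
; It adds HealAmount, calls Respawn, then caps Health at 100.
; Respawn hides the mesh and disables collision, restoring both after RespawnTime.
; The kit destroys itself only when a heal reaches the cap with CanRespawn off; otherwise it returns regardless of that flag.
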(event `self.CL_Medkit_PickupArea.OnComponentBeginOverlap`
  (params (OverlappedComponent :type "PrimitiveComponent Object Reference") (OtherActor :type "Actor Object Reference") (OtherComp :type "PrimitiveComponent Object Reference") (OtherBodyIndex :type Integer) (bFromSweep :type Boolean) (SweepResult :type "HitResult Structure (by ref)"))
  (bind _asbp_player_base (cast `/Game/Character/Blueprints/BP_Player_Base` OtherActor))
  (bind _health (`/Game/Character/Blueprints/BP_Player_Base.Health` _asbp_player_base))
  (if (not (== _health 100.0))
    (bind _output_get (set `/Game/Character/Blueprints/BP_Player_Base.Health` (+ _health (`self.Heal Amount`)) _asbp_player_base))
    (`KismetSystemLibrary.PrintString` (`KismetStringLibrary.Conv_DoubleToString` _output_get) true true (struct :`R` 0.159905 :`G` 0.347249 :`A` 1.0))
    (`self.Respawn`)
    (if (>= _output_get 100.0)
      (set `/Game/Character/Blueprints/BP_Player_Base.Health` 100.0 _asbp_player_base)
      (if (not (`self.Can Respawn ?`))
        (`self.K2_DestroyActor`)
        (`KismetSystemLibrary.PrintString` "destroy")))))

(event `Respawn`
  (`KismetSystemLibrary.PrintString` "Hello")
  (`SceneComponent.SetVisibility` (`self.Medkit`) false false)
  (`PrimitiveComponent.SetCollisionEnabled` (`self.CL_Medkit_PickupArea`) "NoCollision")
  (`KismetSystemLibrary.Delay` (`self.Respawn Time`))
  (`SceneComponent.SetVisibility` (`self.Medkit`) true false)
  (`PrimitiveComponent.SetCollisionEnabled` (`self.CL_Medkit_PickupArea`) "QueryAndPhysics"))

(fn `UserConstructionScript`)